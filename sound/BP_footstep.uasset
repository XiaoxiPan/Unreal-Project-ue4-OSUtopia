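; BP_footstep is a Blueprint that plays a running-shoe footstep sound while the Y key is held.
; BeginPlay assigns the sound cue to the Audio component, then pressing Y plays it and releasing Y stops it.
; Unconnected leftover nodes hold an axis-value check, an AxisMove flag and a PlaySoundAtLocation call, none of which run.
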(event `self.ReceiveBeginPlay`
  (`AudioComponent.SetSound` (`self.audio`) "/Game/FirstPersonBP/sound/151226__owlstorm__running-shoes-1_Cue.151226__owlstorm__running-shoes-1_Cue"))

(event `Key|Y`
  (params (Key :type "Key Structure"))
  (bind _audio (`self.audio`))
  (:`Pressed`
    (`AudioComponent.Play` _audio 0.0))
  (:`Released`
    (`AudioComponent.Stop` _audio)))

(fn `UserConstructionScript`)