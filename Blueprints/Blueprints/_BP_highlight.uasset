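; Interactable actor Blueprint that highlights on mouse hover and shows a subtitle (Zimu) text.
; Cursor over and end toggle custom depth on the static mesh, while a click during hover or a Box overlap triggers the Zimu graph.
; Zimu creates a temporary viewport widget removed after a delay, or only swaps the text if one already exists.
; A DoOnce sound-playback chain is present but never runs.
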(event `self.ReceiveActorBeginCursorOver`
  (set `self.cursorover` true)
  (`PrimitiveComponent.SetRenderCustomDepth` (`self.StaticMesh`) true))

(event `self.ReceiveActorEndCursorOver`
  (set `self.cursorover` false)
  (`PrimitiveComponent.SetRenderCustomDepth` (`self.StaticMesh`) false))

(event `self.ReceiveActorOnClicked`
  (params (ButtonPressed :type "Key Structure"))
  (if (`self.cursorover`)
    (`self.Zimu` (`self.text`) 2.0 :!label _label)))

(event `self.Box.OnComponentBeginOverlap`
  (params (OverlappedComponent :type "PrimitiveComponent Object Reference") (OtherActor :type "Actor Object Reference") (OtherComp :type "PrimitiveComponent Object Reference") (OtherBodyIndex :type Integer) (bFromSweep :type Boolean) (SweepResult :type "HitResult Structure (by ref)"))
  (goto _label))

(fn `UserConstructionScript`)