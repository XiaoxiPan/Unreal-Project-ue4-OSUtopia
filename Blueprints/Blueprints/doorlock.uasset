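; Door lock actor Blueprint that plays the Doorlock sound when the player clicks on it.
; The click event only proceeds while the Cursorover flag is true, and this graph never sets that flag.
; A DoOnce gate resets after a short delay to throttle repeat clicks, and the sound plays at the actor's eyes view point.
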(event `self.ReceiveBeginPlay`
  (`parent.ReceiveBeginPlay`))

(event `self.ReceiveActorOnClicked`
  (params (ButtonPressed :type "Key Structure"))
  ;[1 1 1] sound
  (if (`self.cursorover`)
    (`/Engine/EditorBlueprintResources/StandardMacros.DoOnce` false :!label _label
      (:`Completed`
        (`GameplayStatics.PlaySoundAtLocation` "/Game/myResourse/sound/doorlock.doorlock" (`self.GetActorEyesViewPoint`) (struct) 1.0 1.0 0.0 null null null)
        (`KismetSystemLibrary.Delay` 0.25)
        (goto _label :!via `Reset`)))))

(fn `UserConstructionScript`
  (`parent.UserConstructionScript`))